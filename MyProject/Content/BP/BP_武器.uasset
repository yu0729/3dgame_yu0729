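; BP_武器 is a weapon Blueprint that handles automatic fire and magazine reloading.
; Holding the 開槍 (fire) input runs a Delay-paced loop until release or an empty magazine.
; Each shot spawns an actor at the weapon mesh's 子彈插槽 socket, plays a muzzle flash and decrements loaded ammo.
; The 換彈閘 (reload) event refills the magazine from reserve ammo, capped by what remains.
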(event Custom|換彈閘
  ;[0.2793 0.7302 0.2499] 計算要補充幾顆子彈
  (Variables|Default|Set要補充的子彈數量 (- (Variables|Default|Get彈閘尺寸) (Variables|Default|Get目前子彈數量)))
  ;[0.2767 1 0.1922] 判斷總數是否>=要補充的數量
  (if (>= (Variables|Default|Get子彈總數) (Variables|Default|Get要補充的子彈數量))
    _
    (else
      ;[0.2205 1 0.2696] 總數<要補充的數量:把剩餘總數補充
      (Variables|Default|Set要補充的子彈數量 (Variables|Default|Get子彈總數))))
  ;[0.2799 1 0.354] 目前子彈及總數更新
  (Variables|Default|Set目前子彈數量 (+ (Variables|Default|Get目前子彈數量) (Variables|Default|Get要補充的子彈數量)))
  (Variables|Default|Set子彈總數 (- (Variables|Default|Get子彈總數) (Variables|Default|Get要補充的子彈數量))))

(event Input|ActionEvents|InputAction開槍
  (params (Key :type Key%20Structure :default "None"))
  (bind _武器模型 (Variables|Default|Get武器模型))
  (bind _returnvalue (Transformation|GetSocketRotation _武器模型 "None"))
  ;[1 1 1] 開槍
  (:Pressed
    (Variables|Default|Set開槍中 true)
    (if (and (> (Variables|Default|Get目前子彈數量) 0) (Variables|Default|Get開槍中)) :!label _label
      (Game|SpawnActorfromClass "/Game/BP/BP_子彈.BP_子彈_C" (Transformation|GetSocketTransform (Variables|Default|Get武器模型) "子彈插槽" "RTS_World") "Undefined" 0 0)
      (Effects|SpawnEmitteratLocation "/Game/InfinityBladeEffects/Effects/FX_Monsters/FX_Monster_Gruntling/Master/P_BackPack_MuzzleFlash.P_BackPack_MuzzleFlash" (Transformation|GetSocketLocation _武器模型 "子彈插槽") (Math|Rotator|MakeRotator (+ (.roll _returnvalue) 9e+01) (.pitch _returnvalue) (+ (.yaw _returnvalue) 9e+01)) "0.080000,0.080000,0.080000")
      (Variables|Default|Set目前子彈數量 (- (Variables|Default|Get目前子彈數量) 1))
      (Utilities|FlowControl|Delay (Variables|Default|Get開槍間隔))
      (goto _label)))
  (:Released
    (Variables|Default|Set開槍中 false)))

(fn ConstructionScript)