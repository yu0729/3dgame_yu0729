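; Game mode Blueprint (遊戲模式) that runs a minutes-and-seconds countdown and pauses the game when time runs out.
; Tick feeds a one-second Delay, which throttles the per-frame event to one decrement of the seconds variable (秒) per second.
; When seconds drop below zero, they wrap to 59 and minutes (分) decrease.
; If no minutes remain, seconds reset to zero and the game pauses.
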(event EventTick
  (params (DeltaSeconds :type Float%20%28single-precision%29))
  ;[1 1 1] 倒數系統
  ;;[1 1 1] 每秒秒數減一
  (Utilities|FlowControl|Delay 1.0)
  (bind _output_get (Variables|Default|Set秒 (- (Variables|Default|Get秒) 1)))
  ;;[1 1 1] 當秒數低於0就設成59
  (if (< _output_get 0)
    (Variables|Default|Set秒 59)
    ;;[1 1 1] 分大於0時 分減一
    (if (> (Variables|Default|Get分) 0)
      (Variables|Default|Set分 (- (Variables|Default|Get分) 1))
      (else
        ;;[1 1 1] 時間計算結束
        (if (== (Variables|Default|Get秒) 59)
          (Variables|Default|Set秒 0)
          (Game|SetGamePaused true))))))

(fn ConstructionScript)